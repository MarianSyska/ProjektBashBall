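; Sphere actor that acts as an always-bashable target for a Bash mechanic, reporting its location and priority.
; RegisterBasher adds a BashSocket and a visible, colored Arrow component for each basher, links them, and returns the socket.
; The socket's BashStarted event is bound back to the sphere, which then destroys that socket and its arrow without applying any movement itself.
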(event Custom|BashStarted
  (params (BashDirection :type Vector) (Owner :type Bash%20Socket%20Object%20Reference))
  (Components|DestroyComponent (Variables|/Game/Blueprints/BashSocket.BashSocket_C|GetArrowComponent Owner))
  (Components|DestroyComponent Owner))

(fn ConstructionScript)

(fn GetBashLocation
  (return (Transformation|GetActorLocation)))

(fn GetPriority
  (return (Variables|Default|GetPriority)))

(fn IsBashable
  (return true))

(fn RegisterBasher
  (params (Basher :type Actor%20Object%20Reference) (Color :type Linear%20Color%20Structure))
  (bind _returnvalue (AddComponent|AddBashSocket))
  (LocalVariables|SetBashSocket _returnvalue)
  (bind _returnvalue_2 (AddComponent|AddArrowComponent false))
  (LocalVariables|SetArrow _returnvalue_2)
  (Variables|/Game/Blueprints/BashSocket.BashSocket_C|SetBasher (LocalVariables|GetBashSocket) Basher)
  (Rendering|SetVisibility (LocalVariables|GetArrow) true false)
  (Development|SetHiddeninGame (LocalVariables|GetArrow) false false)
  (Variables|/Script/Engine.ArrowComponent|SetArrowSize (LocalVariables|GetArrow) (Variables|Default|GetArrowSize))
  (Components|Arrow|SetArrowColor(LinearColor) (LocalVariables|GetArrow) Color)
  (Variables|/Game/Blueprints/BashSocket.BashSocket_C|SetArrowComponent (LocalVariables|GetBashSocket) (LocalVariables|GetArrow))
  (EventDispatchers|BindEventtoBashStarted (LocalVariables|GetBashSocket) (EventDispatchers|CreateEvent :!event Custom|BashStarted))
  (return (LocalVariables|GetBashSocket)))