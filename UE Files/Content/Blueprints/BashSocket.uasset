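; BashSocket is an owned Blueprint, apparently a component, that provides a bash point with a directional arrow.
; SetBashDirection rotates the arrow to face the given direction, or hides it when that vector is near zero.
; GetBashLocation asks the owner for the location through a message call.
; StartBash broadcasts BashStarted with the direction and itself, leaving the bash response to listeners.
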(fn SetBashDirection
  (params (BashDirection :type Vector))
  (if (< (Math|Vector|VectorLengthSquared BashDirection) 0.1)
    (Rendering|SetVisibility (Variables|Default|GetArrowComponent) false false)
    (else
      (Rendering|SetVisibility (Variables|Default|GetArrowComponent) true false)
      (Transformation|SetWorldRotation (Variables|Default|GetArrowComponent) (Math|Conversions|RotationFromXVector BashDirection) false false))))

(fn GetBashLocation
  (bind _location (Class|BashableBP|GetBashLocation(Message) (Components|GetOwner)))
  (return _location))

(fn StartBash
  (params (BashDirection :type Vector))
  (Default|CallBashStarted BashDirection self))