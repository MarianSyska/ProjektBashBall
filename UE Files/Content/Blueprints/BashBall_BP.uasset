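; BashBall is a bashable physics ball that a basher can latch onto and launch.
; RegisterBasher freezes its physics, blocks further bashing and returns a new BashSocket component with a colored direction arrow.
; When the socket's BashStarted fires, the ball destroys socket and arrow, re-enables physics, applies force opposite the bash direction and becomes bashable again.
; Getters expose its location, priority and bashable state.
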(event Custom|BashStarted
  (params (BashDirection :type Vector) (Owner :type Bash%20Socket%20Object%20Reference))
  (Components|DestroyComponent (Variables|/Game/Blueprints/BashSocket.BashSocket_C|GetArrowComponent Owner))
  (Components|DestroyComponent Owner)
  (Physics|SetSimulatePhysics (Variables|Default|GetVisuals) true)
  (Physics|AddForce (Variables|Default|GetVisuals) (* (* (Math|Vector|Normalize BashDirection) (Variables|Default|GetBashImpulse)) -1.0) "None" false)
  (Variables|Default|SetIsBahsable_M true))

(fn ConstructionScript)

(fn GetBashLocation
  (return (Transformation|GetActorLocation)))

(fn GetPriority
  (return (Variables|Default|GetPriority)))

(fn IsBashable
  (return (Variables|Default|GetIsBahsable_M)))

(fn RegisterBasher
  (params (Basher :type Actor%20Object%20Reference) (Color :type Linear%20Color%20Structure))
  (Physics|SetSimulatePhysics (Variables|Default|GetVisuals) false)
  (bind _returnvalue (AddComponent|AddBashSocket))
  (LocalVariables|SetBashSocket _returnvalue)
  (bind _returnvalue_2 (AddComponent|AddArrowComponent false))
  (LocalVariables|SetArrow _returnvalue_2)
  (Variables|/Script/Engine.ArrowComponent|SetArrowSize (LocalVariables|GetArrow) (Variables|Default|GetArrowSize))
  (Rendering|SetVisibility (LocalVariables|GetArrow) true false)
  (Development|SetHiddeninGame (LocalVariables|GetArrow) false false)
  (Components|Arrow|SetArrowColor(LinearColor) (LocalVariables|GetArrow) Color)
  (Variables|/Game/Blueprints/BashSocket.BashSocket_C|SetArrowComponent (LocalVariables|GetBashSocket) (LocalVariables|GetArrow))
  (Variables|/Game/Blueprints/BashSocket.BashSocket_C|SetBasher (LocalVariables|GetBashSocket) Basher)
  (EventDispatchers|BindEventtoBashStarted (LocalVariables|GetBashSocket) (EventDispatchers|CreateEvent :!event Custom|BashStarted))
  (Variables|Default|SetIsBahsable_M false)
  (return (LocalVariables|GetBashSocket)))